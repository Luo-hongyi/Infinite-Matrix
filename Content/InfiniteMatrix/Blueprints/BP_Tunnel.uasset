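; BP_Tunnel is an endless-runner tunnel segment with a rotating holed wall, a health pickup and an enemy.
; Randomize functions vary meshes, rotation, offsets and pickup presence.
; Overlaps drive gameplay: wall and enemy damage the player, pickups heal, and projectiles are destroyed, killing enemies and rewarding the shooter with health.
; The trigger zone asks TunnelSpawner for another segment, destroys this one and scores if the wall was avoided.
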(event OnComponentBeginOverlap(TriggerZone)
  (params (OverlappedComponent :type Primitive%20Component%20Object%20Reference) (OtherActor :type Actor%20Object%20Reference) (OtherComp :type Primitive%20Component%20Object%20Reference) (OtherBodyIndex :type Integer) (bFromSweep :type Boolean) (SweepResult :type Hit%20Result%20Structure%20%28by%20ref%29))
  (bind _asbp_player (Utilities|Casting|CastToBP_Player OtherActor))
  (Default|SpawnTunnelatSpawnPoint (Variables|Default|GetTunnelSpawner))
  (Actor|DestroyActor)
  (if (not (Variables|Default|GetHitWall))
    (Default|ChangeScore _asbp_player 1)
    (Variables|Default|SetHitWall false)))

(event OnComponentBeginOverlap(WallMesh)
  (params (OverlappedComponent :type Primitive%20Component%20Object%20Reference) (OtherActor :type Actor%20Object%20Reference) (OtherComp :type Primitive%20Component%20Object%20Reference) (OtherBodyIndex :type Integer) (bFromSweep :type Boolean) (SweepResult :type Hit%20Result%20Structure%20%28by%20ref%29))
  (bind _asbp_player (Utilities|Casting|CastToBP_Player OtherActor)
    (:then
      (Utilities|FlowControl|Sequence
        (:then_0
          (bind _returnvalue (UserInterface|CreateWidget "/Game/InfiniteMatrix/UI/WB_RedScreen.WB_RedScreen_C"))
          (UserInterface|Viewport|AddtoViewport _returnvalue 0))
        (:then_1
          (bind _newhealth (Default|ChangeHealth _asbp_player -2e+01))
          (Variables|Default|SetHitWall true)
          (if (<= _newhealth 0.0)
            (Variables|/Game/InfiniteMatrix/Blueprints/BP_Player.BP_Player_C|SetIsDead _asbp_player true)
            (Default|DisplayRestart _asbp_player)))))
    (:CastFailed
      (bind _asbp_projectile (Utilities|Casting|CastToBP_Projectile OtherActor))
      (Actor|DestroyActor _asbp_projectile))))

(event OnComponentBeginOverlap(HealthKit)
  (params (OverlappedComponent :type Primitive%20Component%20Object%20Reference) (OtherActor :type Actor%20Object%20Reference) (OtherComp :type Primitive%20Component%20Object%20Reference) (OtherBodyIndex :type Integer) (bFromSweep :type Boolean) (SweepResult :type Hit%20Result%20Structure%20%28by%20ref%29))
  (bind _asbp_player (Utilities|Casting|CastToBP_Player OtherActor)
    (:then
      (Default|ChangeHealth _asbp_player 1e+01)
      (Components|DestroyComponent (Variables|Default|GetHealthKit))
      (bind _returnvalue (UserInterface|CreateWidget "/Game/InfiniteMatrix/UI/WB_HealthKitIndicator.WB_HealthKitIndicator_C"))
      (UserInterface|Viewport|AddtoViewport _returnvalue 0))
    (:CastFailed
      (bind _asbp_projectile (Utilities|Casting|CastToBP_Projectile OtherActor))
      (Actor|DestroyActor _asbp_projectile))))

(event OnComponentBeginOverlap(Enemy)
  (params (OverlappedComponent :type Primitive%20Component%20Object%20Reference) (OtherActor :type Actor%20Object%20Reference) (OtherComp :type Primitive%20Component%20Object%20Reference) (OtherBodyIndex :type Integer) (bFromSweep :type Boolean) (SweepResult :type Hit%20Result%20Structure%20%28by%20ref%29))
  (bind _asbp_player (Utilities|Casting|CastToBP_Player OtherActor)
    (:then
      (bind _newhealth (Default|ChangeHealth _asbp_player -1e+01))
      (if (> _newhealth 0.0)
        (Components|DestroyComponent (Variables|Default|GetEnemy))
        (else
          (Variables|/Game/InfiniteMatrix/Blueprints/BP_Player.BP_Player_C|SetIsDead _asbp_player true)
          (Default|DisplayRestart _asbp_player))))
    (:CastFailed
      (bind _asbp_projectile (Utilities|Casting|CastToBP_Projectile OtherActor))
      (if (Utilities|IsValid _asbp_projectile)
        (Utilities|FlowControl|Sequence
          (:then_0
            (bind _shootfrom (Default|GetShootfromPlayer _asbp_projectile))
            (if (Utilities|IsValid _shootfrom)
              (Default|ChangeHealth _shootfrom 5.0)))
          (:then_1
            (Actor|DestroyActor _asbp_projectile))
          (:then_2
            (Components|DestroyComponent (Variables|Default|GetEnemy))))))))

(event EventBeginPlay)

(event EventTick
  (params (DeltaSeconds :type Float%20%28single-precision%29))
  (bind _rotatespeed (Variables|Default|GetRotateSpeed))
  (bind _healthkit (Variables|Default|GetHealthKit))
  (bind _returnvalue (* DeltaSeconds _rotatespeed))
  (Transformation|AddLocalRotation (Variables|Default|GetWallMesh) (Math|Rotator|MakeRotator _returnvalue 0.0 0.0) false false)
  (if (Utilities|IsValid _healthkit)
    (Transformation|AddLocalRotation _healthkit (Math|Rotator|MakeRotator 0.0 0.0 _returnvalue) false false)))

(fn ConstructionScript)

(fn RandomizeWall
  (Components|StaticMesh|SetStaticMesh (Variables|Default|GetWallMesh) (Utilities|Select :Index (Math|Random|RandomIntegerinRange 0 3) :Option%200 "/Game/InfiniteMatrix/Meshes/SM_Hole_01.SM_Hole_01" :Option%201 "/Game/InfiniteMatrix/Meshes/SM_Hole_02.SM_Hole_02" :Option%202 "/Game/InfiniteMatrix/Meshes/SM_Hole_03.SM_Hole_03" :Option%203 "/Game/InfiniteMatrix/Meshes/SM_Hole_04.SM_Hole_04"))
  (Transformation|AddLocalRotation (Variables|Default|GetWallMesh) (Math|Rotator|MakeRotator (Math|Random|RandomFloatinRange 0.0 3.6e+02) 0.0 0.0) false false))

(fn RandomizeHealthKits
  (Components|StaticMesh|SetStaticMesh (Variables|Default|GetHealthKit) (Utilities|Select :Index (Math|Random|RandomIntegerinRange 0 3) :Option%200 "/Game/InfiniteMatrix/FirstAid/SM_FirstAidKit.SM_FirstAidKit" :Option%201 "/Game/InfiniteMatrix/Health/SM_Apple_Leafy.SM_Apple_Leafy" :Option%202 "/Game/InfiniteMatrix/Health/SM_Banana_Bunch.SM_Banana_Bunch" :Option%203 "/Game/InfiniteMatrix/Health/SM_Kiwi_Half.SM_Kiwi_Half"))
  (Transformation|AddLocalOffset (Variables|Default|GetHealthKit) (Math|Vector|MakeVector (Math|Random|RandomFloatinRange -5e+02 5e+02) (Math|Random|RandomFloatinRange -5e+01 5e+01) (Math|Random|RandomFloatinRange -5e+01 5e+01)) false false))

(fn RandomizeHealthKit
  (bind _healthkit (Variables|Default|GetHealthKit))
  (if (>= (Math|Random|RandomIntegerinRange 0 9) 5)
    (Components|DestroyComponent _healthkit)
    (else
      (Transformation|AddLocalOffset _healthkit (Math|Vector|MakeVector (Math|Random|RandomFloatinRange -5e+02 5e+02) (Math|Random|RandomFloatinRange -2e+02 2e+02) (Math|Random|RandomFloatinRange -2e+02 2e+02)) false false))))

(fn RandomizeEnemy
  (Transformation|AddLocalOffset (Variables|Default|GetEnemy) (Math|Vector|MakeVector (Math|Random|RandomFloatinRange -1e+02 2e+02) (Math|Random|RandomFloatinRange -1.2e+02 1.2e+02) (Math|Random|RandomFloatinRange -1.2e+02 1.2e+02)) false false))